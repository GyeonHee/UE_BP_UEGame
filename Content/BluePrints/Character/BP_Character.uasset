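; Player character Blueprint with Enhanced Input movement, mouse look and a melee-style attack.
; BeginPlay adds the character mapping context; look input drives controller rotation, and move input follows control rotation, using only yaw for forward movement.
; Attack switches a Peace/Battle state and plays the attack montage's first section, ignoring further presses until AttackEnd restores Peace.
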(event Custom|Attack
  (switch Utilities|FlowControl|Switch|SwitchonECharacterState (Variables|Default|GetState_BP)
    (:NewEnumerator0
      (Variables|Default|SetState_BP "NewEnumerator1")
      (Animation|PlayAnimMontage "/Game/InfinityBladeWarriors/Characters/AM_CharacterAttack.AM_CharacterAttack" 1.0 "Attack1"))))

(event Custom|AttackEnd
  (Variables|Default|SetState_BP "NewEnumerator0"))

(event Input|EnhancedActionEvents|EnhancedInputActionIA_Move
  (params (ActionValue :type Vector%202D%20Structure) (ElapsedSeconds :type Float%20%28double-precision%29) (TriggeredSeconds :type Float%20%28double-precision%29) (InputAction :type Input%20Action%20Object%20Reference :default "/Game/BluePrints/Inputs/Actions/IA_Move.IA_Move"))
  ;[0.15 0.15 0.15 0.5] IA_Move
  (Pawn|Input|AddMovementInput (* (Math|Vector|GetForwardVector (Math|Rotator|MakeRotator 0.0 0.0 (.yaw (Pawn|GetControlRotation :!class /Script/Engine.Pawn)))) (.y ActionValue)) 1.0 false)
  (Pawn|Input|AddMovementInput (* (Math|Vector|GetRightVector (Pawn|GetControlRotation :!class /Script/Engine.Pawn)) (.x ActionValue)) 1.0 false))

(event Input|EnhancedActionEvents|EnhancedInputActionIA_Look
  (params (ActionValue :type Vector%202D%20Structure) (ElapsedSeconds :type Float%20%28double-precision%29) (TriggeredSeconds :type Float%20%28double-precision%29) (InputAction :type Input%20Action%20Object%20Reference :default "/Game/BluePrints/Inputs/Actions/IA_Look.IA_Look"))
  ;[0.15 0.15 0.15 0.5] 마우스 입력을 컨트롤러 회전에 적용
  (Pawn|Input|AddControllerYawInput (.x ActionValue))
  (Pawn|Input|AddControllerPitchInput (.y ActionValue)))

(event Input|EnhancedActionEvents|EnhancedInputActionIA_Attack
  (params (ActionValue :type Boolean) (ElapsedSeconds :type Float%20%28double-precision%29) (TriggeredSeconds :type Float%20%28double-precision%29) (InputAction :type Input%20Action%20Object%20Reference :default "/Game/BluePrints/Inputs/Actions/IA_Attack.IA_Attack"))
  (CallFunction|Attack))

(event EventBeginPlay
  ;[0.15 0.15 0.15 0.5] Input Controller
  (Input|AddMappingContext (PlayerController|LocalPlayerSubsystems|GetEnhancedInputLocalPlayerSubsystem (Game|GetPlayerController 0)) "/Game/BluePrints/Inputs/IMC_Character.IMC_Character" 0 "(bIgnoreAllPressedKeysUntilRelease=True,bForceImmediately=False,bNotifyUserSettings=False)"))

(event Collision|EventActorBeginOverlap
  (params (OtherActor :type Actor%20Object%20Reference)))

(event EventTick
  (params (DeltaSeconds :type Float%20%28single-precision%29)))

(fn ConstructionScript)